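; BP_Barrel is a physics barrel that characters pick up and throw, and that is destroyed by any damage.
; PickedUp snaps it to the GripPoint socket on the character's first-person mesh and disables physics and collision.
; Throw calls detach through the attach parent actor, then restores physics and collision without applying an impulse itself.
; Impacts above a threshold play random bounce sounds, only where cosmetic events can execute.
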(event `self.ReceiveAnyDamage`
  (params (Damage :type "Float (single-precision)") (DamageType :type "DamageType Object Reference") (InstigatedBy :type "Controller Object Reference") (DamageCauser :type "Actor Object Reference"))
  (`self.K2_DestroyActor`))

(event `self.ReceiveHit`
  (params (MyComp :type "PrimitiveComponent Object Reference") (Other :type "Actor Object Reference") (OtherComp :type "PrimitiveComponent Object Reference") (bSelfMoved :type Boolean) (HitLocation :type "Vector Structure") (HitNormal :type "Vector Structure") (NormalImpulse :type "Vector Structure") (Hit :type "HitResult Structure (by ref)"))
  (`/Engine/EditorBlueprintResources/StandardMacros.Can Execute Cosmetic Events`
    (:`True`
      (if (> (`KismetMathLibrary.VSize` NormalImpulse) (`self.SoundThreshold`))
        (`GameplayStatics.PlaySoundAtLocation` (`KismetArrayLibrary.Array_Random` (`self.BounceSounds`)) HitLocation (struct) 1.0 1.0 0.0 null null null null)))))

(fn `Picked Up`
  (params (Character :type "/Game/Blueprints/FirstPerson/Blueprints/BP_FirstPersonCharacter Object Reference"))
  (bind _staticmesh (`self.StaticMesh`))
  (`self.K2_AttachToComponent` (`/Game/Blueprints/FirstPerson/Blueprints/BP_FirstPersonCharacter.FirstPersonMesh` Character) "GripPoint" "SnapToTarget" "SnapToTarget" "SnapToTarget")
  (`PrimitiveComponent.SetSimulatePhysics` _staticmesh false)
  (`PrimitiveComponent.SetCollisionEnabled` _staticmesh "NoCollision"))

(fn `Throw`
  (bind _staticmesh (`self.StaticMesh`))
  (`self.K2_DetachFromActor` (`self.GetAttachParentActor`) "KeepWorld" "KeepWorld" "KeepWorld")
  (`PrimitiveComponent.SetSimulatePhysics` _staticmesh true)
  (`PrimitiveComponent.SetCollisionEnabled` _staticmesh "QueryAndPhysics"))

(fn `UserConstructionScript`)