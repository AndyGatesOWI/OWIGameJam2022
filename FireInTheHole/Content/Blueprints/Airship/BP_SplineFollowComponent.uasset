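; Actor component in the Airship folder that flies its owner along the spline of the nearest BP_SplineTarget, found once at BeginPlay.
; Each tick it projects a look-ahead point along the owner's forward vector and takes the closest spline location as the movement target, with debug drawing.
; It then moves the owner along local X at scaled max speed and snaps its rotation toward that target.
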(event `self.ReceiveBeginPlay`
  (`self.FindSplineTarget`))

(event `self.ReceiveTick`
  (params (DeltaSeconds :type "Float (single-precision)"))
  (`self.UpdateMovementTarget`)
  (`self.PerformMovement` DeltaSeconds))

(fn `FindSplineTarget`
  (bind _outactors (`GameplayStatics.GetAllActorsOfClass` "/Game/Blueprints/Airship/BP_SplineTarget.BP_SplineTarget_C"))
  (bind _asbp_spline_target (cast `/Game/Blueprints/Airship/BP_SplineTarget` (`.ReturnValue` (`GameplayStatics.FindNearestActor` (`Actor.K2_GetActorLocation` (`self.GetOwner`)) _outactors)))
    (:`then`
      _)
    (:`CastFailed`
      _))
  (set `self.SplineTarget` _asbp_spline_target))

(fn `PerformMovement`
  (params (DeltaTime :type "Float (double-precision)"))
  (bind _returnvalue (`self.GetOwner`))
  (`Actor.K2_AddActorLocalOffset` _returnvalue (`KismetMathLibrary.MakeVector` (* DeltaTime (* (`self.MaxSpeed`) (`self.SpeedMultiplier`)))) false false)
  (`Actor.K2_SetActorRotation` (`self.GetOwner`) (`KismetMathLibrary.FindLookAtRotation` (`SceneComponent.K2_GetComponentLocation` (`Actor.RootComponent` _returnvalue)) (`self.MovementTarget`)) false))

(fn `UpdateMovementTarget`
  (locals (SearchOffset :type "Float (double-precision)" :default 100.0))
  (bind _returnvalue (`self.GetOwner`))
  (bind _output_get (set `self.MovementTarget` (`SplineComponent.FindLocationClosestToWorldLocation` (`/Game/Blueprints/Airship/BP_SplineTarget.Spline` (`self.SplineTarget`)) (+ (`Actor.K2_GetActorLocation` _returnvalue) (* (`Actor.GetActorForwardVector` _returnvalue) (`local.SearchOffset`))) "World")))
  (`KismetSystemLibrary.DrawDebugSphere` _output_get)
  (`KismetSystemLibrary.DrawDebugString` (0.0 0.0 0.0) (`KismetStringLibrary.Conv_VectorToString` _output_get) null))