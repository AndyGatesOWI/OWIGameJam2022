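; Template game mode that handles player respawning and end-of-match restarts.
; Respawn spawns the default pawn at the respawn point of a randomly chosen BP_Airship and possesses it with the given controller.
; OnEndGame calls OnGameOver on the template player controllers found through the game state's player array, then after a short delay server-travels to the current level to restart it.
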(event `Respawn`
  (params (PC :type "PlayerController Object Reference"))
  (bind _outactors (`GameplayStatics.GetAllActorsOfClass` "/Game/Blueprints/Airship/BP_Airship.BP_Airship_C"))
  (bind _returnvalue (`|SpawnActorFromClass` (`self.DefaultPawnClass`) (`SceneComponent.K2_GetComponentToWorld` (`/Game/Blueprints/Airship/BP_Airship.RespawnPoint` (`KismetArrayLibrary.Array_Random` _outactors))) "Undefined" "OverrideRootScale" null null))
  (`Controller.Possess` PC _returnvalue))

(event `OnEndGame`
  (for _array_element (`GameStateBase.PlayerArray` (`GameplayStatics.GetGameState`))
    (bind _asbp_player_controller_template (cast `/Game/Blueprints/Core/BP_PlayerController_Template` (`PlayerState.GetPlayerController` _array_element)))
    (`/Game/Blueprints/Core/BP_PlayerController_Template.OnGameOver` _asbp_player_controller_template))
  (`KismetSystemLibrary.Delay` 5.0)
  (bind _returnvalue (`GameplayStatics.GetCurrentLevelName` true))
  (`AdvancedSessionsLibrary.ServerTravel` _returnvalue))

(fn `UserConstructionScript`)