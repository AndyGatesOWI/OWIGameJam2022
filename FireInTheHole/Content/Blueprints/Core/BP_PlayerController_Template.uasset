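; Template player controller that forwards menu input, respawn requests and game-over events to other framework classes.
; The Menu input action toggles the menu on BP_HUD_Template.
; Respawn passes the controller itself to BP_GameMode_Template, which performs the respawn.
; OnGameOver tells the HUD to show the game-over screen, with each call going through a cast that silently stops on failure.
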(event `InputAction|Menu`
  (params (Key :type "Key Structure"))
  ;[1 1 1] Open and Close Menu
  (:`Pressed`
    (bind _asbp_hud_template (cast `/Game/Blueprints/Core/BP_HUD_Template` (`self.GetHUD`)))
    (`/Game/Blueprints/Core/BP_HUD_Template.Toggle Menu` _asbp_hud_template)))

(event `Respawn`
  (bind _asbp_game_mode_template (cast `/Game/Blueprints/Core/BP_GameMode_Template` (`GameplayStatics.GetGameMode`)))
  (`/Game/Blueprints/Core/BP_GameMode_Template.Respawn` _asbp_game_mode_template self))

(event `OnGameOver`
  (bind _asbp_hud_template (cast `/Game/Blueprints/Core/BP_HUD_Template` (`self.GetHUD`)))
  (`/Game/Blueprints/Core/BP_HUD_Template.ShowGameOver` _asbp_hud_template))

(fn `UserConstructionScript`)