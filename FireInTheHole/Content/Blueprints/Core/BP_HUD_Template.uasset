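; Template HUD Blueprint that creates and controls the menu, tutorial and game-over widgets.
; On BeginPlay it adds all three to the viewport, with the menu and game-over screens collapsed and the tutorial at a higher Z-order.
; ToggleMenu flips menu visibility, switching input mode and mouse cursor between game-only and UI-only.
; ShowGameOver reveals the game-over screen with UI-only input and a visible cursor.
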(event `self.ReceiveBeginPlay`
  (`self.Create Menu`)
  (`self.Create Tutorial`)
  (`self.CreateGameOver`))

(event `Create Menu`
  (bind _returnvalue (`GameplayStatics.GetPlayerController` 0))
  (bind _returnvalue_2 (`|CreateWidget` "/Game/UserInterface/W_Menu.W_Menu_C"))
  (bind _output_get (set `self.Menu` _returnvalue_2))
  (`UserWidget.AddToViewport` _output_get 9990)
  (`Widget.SetVisibility` _output_get "Collapsed")
  (`WidgetBlueprintLibrary.SetInputMode_GameOnly` _returnvalue)
  (set `PlayerController.bShowMouseCursor` false _returnvalue))

(event `Toggle Menu`
  (bind _returnvalue (`GameplayStatics.GetPlayerController` 0))
  ;[1 1 1] Show and Hide Menu
  (bind _menu (`self.Menu`)
    (:`then`
      (if (`Widget.IsVisible` _menu)
        (`Widget.SetVisibility` (`self.Menu`) "Collapsed")
        (`WidgetBlueprintLibrary.SetInputMode_GameOnly` _returnvalue)
        (set `PlayerController.bShowMouseCursor` false _returnvalue)
        (else
          (`Widget.SetVisibility` (`self.Menu`) "Visible")
          (`WidgetBlueprintLibrary.SetInputMode_UIOnlyEx` _returnvalue (`self.Menu`))
          (set `PlayerController.bShowMouseCursor` true _returnvalue))))
    (:`else`)))

(event `Create Tutorial`
  (bind _returnvalue (`|CreateWidget` "/Game/UserInterface/W_Tutorial.W_Tutorial_C"))
  (`UserWidget.AddToViewport` _returnvalue 9999))

(event `CreateGameOver`
  (bind _returnvalue (`|CreateWidget` "/Game/UserInterface/W_GameOver.W_GameOver_C"))
  (bind _output_get (set `self.GameOver` _returnvalue))
  (`UserWidget.AddToViewport` _output_get 9990)
  (`Widget.SetVisibility` _output_get "Collapsed"))

(event `ShowGameOver`
  (bind _returnvalue (`GameplayStatics.GetPlayerController` 0))
  (bind _gameover (`self.GameOver`)
    (:`then`
      (`Widget.SetVisibility` _gameover "Visible")
      (`WidgetBlueprintLibrary.SetInputMode_UIOnlyEx` _returnvalue (`self.GameOver`))
      (set `PlayerController.bShowMouseCursor` true _returnvalue))
    (:`else`)))

(fn `UserConstructionScript`)